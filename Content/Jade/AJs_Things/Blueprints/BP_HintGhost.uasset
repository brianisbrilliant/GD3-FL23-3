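; BP_HintGhost is a ghost actor that shows the player a hint by travelling from a HintStart actor to a HintEnd actor.
; GiveHint turns the mesh toward HintEnd, teleports to HintStart and uses AI MoveTo, with a timeline lerp of the mesh if the move aborts.
; Afterwards it teleports back to the capsule location saved at BeginPlay.
; Player attachment, hiding and bobbing logic is left unconnected.
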(event `self.ReceiveBeginPlay`
  (set `self.RecycleLoc` (`SceneComponent.K2_GetComponentLocation` (`self.CapsuleComponent`))))

(event `self.ReceiveTick`
  (params (DeltaSeconds :type "Float (single-precision)")))

(event `GiveHint`
  (`|ExecutionSequence`
    (:`then_0`
      (`self.SetFacingDirection`)
      (`self.K2_SetActorLocation` (`self.K2_GetActorLocation` (`self.HintStart`)))
      (`KismetSystemLibrary.Delay` 0.5)
      (bind _movementresult (`|AIMoveTo` self (`self.K2_GetActorLocation` (`self.HintEnd`)) null)
        (:`OnSuccess`
          (`KismetSystemLibrary.Delay` 0.5 :!label _label)
          (`self.K2_SetActorLocation` (`self.RecycleLoc`))
          (`KismetSystemLibrary.PrintString` "I Should be home now"))
        (:`OnFail`
          (switch `EPathFollowingResult` _movementresult
            (:`Aborted`
              (bind (_direction _moveposition) (`Timeline|MoveTo` :!via `PlayFromStart`)
                (:`Update`
                  (`SceneComponent.K2_SetWorldLocation` (`self.Mesh`) (`KismetMathLibrary.VLerp` (`SceneComponent.K2_GetComponentLocation` (`Actor.RootComponent` (`self.HintStart`))) (`SceneComponent.K2_GetComponentLocation` (`Actor.RootComponent` (`self.HintEnd`))) _moveposition) false false))
                (:`Finished`
                  (goto _label))))))))))

(event `SetFacingDirection`
  (`SceneComponent.K2_SetRelativeRotation` (`self.Mesh`) (`KismetMathLibrary.FindLookAtRotation` (`self.K2_GetActorLocation`) (`self.K2_GetActorLocation` (`self.HintEnd`))) false false))

(fn `UserConstructionScript`)