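; BP_HintTrigger is a trigger volume that has a referenced hint ghost give a hint between its start and end locations.
; Overlap hides a candle flame, marks the trigger as used and starts a cooldown, after which the flame returns.
; An optional NextHint reference chains triggers: once the next one has been triggered, this one stops giving hints and its flame stays hidden after cooldown.
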(event `self.TriggerVolume.OnComponentBeginOverlap`
  (params (OverlappedComponent :type "PrimitiveComponent Object Reference") (OtherActor :type "Actor Object Reference") (OtherComp :type "PrimitiveComponent Object Reference") (OtherBodyIndex :type Integer) (bFromSweep :type Boolean) (SweepResult :type "HitResult Structure (by ref)"))
  (if (not (`self.OnCooldown`))
    (`/Engine/EditorBlueprintResources/StandardMacros.DoOnce` false :!label _label
      (:`Completed`
        (`|ExecutionSequence`
          (:`then_0`
            (`self.Cooldown`))
          (:`then_1`
            (`self.UpdateHintLocation`)
            (`self.CallForHint`)
            (set `self.OnCooldown` true)
            (goto _label :!via `Reset`)))))))

(event `CooldownTimer`
  (`/Engine/EditorBlueprintResources/StandardMacros.DoOnce` false :!label _label_2
    (:`Completed`
      (`KismetSystemLibrary.Delay` (`self.CooldownPeriod`))
      (set `self.OnCooldown` false)
      (`self.ResetHint`)
      (goto _label_2 :!via `Reset`))))

(event `Cooldown`
  (`KismetSystemLibrary.PrintString` "On Cooldown")
  (`|ExecutionSequence`
    (:`then_0`
      (`self.CooldownTimer`))
    (:`then_1`
      (`SceneComponent.SetVisibility` (`self.FX_CandleFlame_01`) false true))
    (:`then_2`
      (`/Engine/EditorBlueprintResources/StandardMacros.DoOnce` false
        (:`Completed`
          (set `self.HasBeenTriggered` true))))))

(event `ResetHint`
  (`self.IsNextHintValid`)
  (if true
    (if (not (`/Game/Jade/AJs_Things/Blueprints/BP_HintTrigger.HasBeenTriggered` (`self.NextHint`)))
      (`SceneComponent.SetVisibility` (`self.FX_CandleFlame_01`) true true))
    (else
      (`SceneComponent.SetVisibility` (`self.FX_CandleFlame_01`) true true))))

(event `CallForHint`
  (`self.IsNextHintValid`)
  (if true
    (if (not (`/Game/Jade/AJs_Things/Blueprints/BP_HintTrigger.HasBeenTriggered` (`self.NextHint`)))
      (`/Game/Jade/AJs_Things/Blueprints/BP_HintGhost.GiveHint` (`self.HintGhostRef`)))))

(event `UpdateHintLocation`
  (bind _hintghostref (`self.HintGhostRef`))
  (set `/Game/Jade/AJs_Things/Blueprints/BP_HintGhost.HintStart` (`self.HintStartLoc`) _hintghostref)
  (set `/Game/Jade/AJs_Things/Blueprints/BP_HintGhost.HintEnd` (`self.HintEndLoc`) _hintghostref))

(fn `IsNextHintValid`
  (returns (`Return Value` :type Boolean))
  (`/Engine/EditorBlueprintResources/StandardMacros.IsValid` (`self.NextHint`)
    (:`Is Valid`
      (return true))
    (:`Is Not Valid`
      (return false))))

(fn `UserConstructionScript`)