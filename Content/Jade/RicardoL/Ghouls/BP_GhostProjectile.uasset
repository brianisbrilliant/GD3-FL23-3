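; BP_GhostProjectile is a projectile that damages ghoul enemies.
; When Sphere1 overlaps a BP_Enemy_Ghoul, it decrements that ghoul's Health and calls StopGhoul once Health reaches zero or below, without destroying itself.
; On hitting a physics-simulating component, it applies an impulse from its velocity, scaled to zero so it imparts no push, then destroys itself.
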(event `self.ReceiveHit`
  (params (MyComp :type "PrimitiveComponent Object Reference") (Other :type "Actor Object Reference") (OtherComp :type "PrimitiveComponent Object Reference") (bSelfMoved :type Boolean) (HitLocation :type "Vector Structure") (HitNormal :type "Vector Structure") (NormalImpulse :type "Vector Structure") (Hit :type "HitResult Structure (by ref)"))
  (if (`SceneComponent.IsSimulatingPhysics` OtherComp "None")
    (`PrimitiveComponent.AddImpulseAtLocation` OtherComp (* (`self.GetVelocity`) (0.0 0.0 0.0)) (`self.K2_GetActorLocation`) "None")
    (`self.K2_DestroyActor`)))

(event `self.Sphere1.OnComponentBeginOverlap`
  (params (OverlappedComponent :type "PrimitiveComponent Object Reference") (OtherActor :type "Actor Object Reference") (OtherComp :type "PrimitiveComponent Object Reference") (OtherBodyIndex :type Integer) (bFromSweep :type Boolean) (SweepResult :type "HitResult Structure (by ref)"))
  (bind _asbp_enemy_ghoul (cast `/Game/Jade/RicardoL/Ghouls/BP_Enemy_Ghoul` OtherActor))
  (bind _health (`/Game/Jade/RicardoL/Ghouls/BP_Enemy_Ghoul.Health` _asbp_enemy_ghoul))
  (`/Engine/EditorBlueprintResources/StandardMacros.DecrementFloat` _health
    (:`  `
      (if (<= _health 0.0)
        (`/Game/Jade/RicardoL/Ghouls/BP_Enemy_Ghoul.Stop Ghoul` _asbp_enemy_ghoul)))))

(fn `UserConstructionScript`)