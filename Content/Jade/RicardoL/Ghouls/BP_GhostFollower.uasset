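; BP_GhostFollower is a ghost companion that follows the BP_Devvy player and fires at nearby ghouls.
; BeginPlay attaches the ghost to the player, while a Tick-called timeline repositions it at a fixed world offset from the player with a looping vertical bob.
; When PawnSensing sees an unstunned BP_Ghoul in range, it turns the mesh toward it and spawns a BP_GhostProjectile after a tiny delay.
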(event `self.ReceiveBeginPlay`
  (set `self.StartWorldRotation` (`SceneComponent.K2_GetComponentRotation` (`self.Mesh`)))
  (bind _asbp_devvy (castclass `/Game/Blueprints/BP_Devvy` "/Game/Blueprints/BP_Devvy.BP_Devvy_C"))
  (bind _returnvalue (`GameplayStatics.GetActorOfClass` _asbp_devvy))
  (bind _output_get (set `self.PlayerRef` _returnvalue))
  (bind _asactor (castclass `Actor` "BP_GhostFollower_C"))
  (bind _returnvalue_2 (`GameplayStatics.GetActorOfClass` _asactor))
  (bind _output_get_2 (set `self.GhostRef` _returnvalue_2))
  (`self.K2_AttachToActor` _output_get_2 _output_get "None" "KeepRelative" "KeepRelative" "KeepRelative" true))

(event `self.ReceiveTick`
  (params (DeltaSeconds :type "Float (single-precision)"))
  (bind (_direction _bobble) (`Timeline|Bobble` :!label _label)
    (:`Update`
      (`self.K2_SetActorLocation` (`self.GhostRef`) (+ (`self.K2_GetActorLocation` (`self.PlayerRef`)) (`KismetMathLibrary.MakeVector` 35.0 90.0 _bobble)) true false))
    (:`Finished`
      (`KismetSystemLibrary.Delay` DeltaSeconds)
      (goto _label :!via `PlayFromStart`))))

(event `self.PawnSensing.OnSeePawn`
  (params (Pawn :type "Pawn Object Reference"))
  (bind _returnvalue (`SceneComponent.K2_GetComponentLocation` (`self.CapsuleComponent`)))
  (bind _asbp_ghoul (cast `/Game/Jade/RicardoL/Ghouls/BP_Ghoul` Pawn))
  (if (not (`/Game/Jade/RicardoL/Ghouls/BP_Ghoul.IsStunned` _asbp_ghoul))
    (bind _returnvalue_2 (`SceneComponent.K2_GetComponentLocation` (`Character.CapsuleComponent` _asbp_ghoul)))
    (bind _returnvalue_3 (<= (`KismetMathLibrary.Vector_Distance` _returnvalue _returnvalue_2) 4000.0))
    (if _returnvalue_3
      (`SceneComponent.K2_SetWorldRotation` (`self.Mesh`) (`KismetMathLibrary.FindLookAtRotation` _returnvalue _returnvalue_2) false false)
      (if _returnvalue_3
        (`KismetSystemLibrary.Delay` 0.001)
        (`|SpawnActorFromClass` "/Game/Jade/RicardoL/Ghouls/BP_GhostProjectile.BP_GhostProjectile_C" (`SceneComponent.K2_GetComponentToWorld` (`self.ProjectileStart`)) "Undefined" "MultiplyWithRoot" null null)))))

(fn `UserConstructionScript`)