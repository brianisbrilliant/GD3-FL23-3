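; BP_Ghoul is an enemy that chases seen pawns and teleports BP_Devvy to a set transform on contact.
; PawnSensing triggers an AI move to the seen pawn's location, clearing the chase flag on success or failure.
; Sphere overlap performs the teleport unless stunned.
; StunGhoul turns the light blue and disables movement and Sphere for a duration, then restores them, the red light and health.
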(event `Stun Ghoul`
  (bind _charactermovement (`self.CharacterMovement`))
  (`LightComponent.SetLightColor` (`self.PointLight`) (struct :`G` 0.164047 :`B` 0.409722 :`A` 1.0) true)
  (`ActorComponent.Deactivate` _charactermovement)
  (`ActorComponent.Deactivate` (`self.Sphere`))
  (set `self.IsStunned` true)
  (`KismetSystemLibrary.Delay` (`self.Stun Duration`))
  (`ActorComponent.Activate` _charactermovement false)
  (`LightComponent.SetLightColor` (`self.PointLight`) (struct :`R` 0.871367 :`B` 0.016893 :`A` 1.0) true)
  (`ActorComponent.Activate` (`self.Sphere`) false)
  (set `self.Health` (`self.ChangableHealth`))
  (set `self.IsStunned` false))

(event `Get Player`
  (set `self.Chaseing Player` true)
  (`|AIMoveTo` self (`self.K2_GetActorLocation` (stale `self.PawnSensing.OnSeePawn` Pawn)) null 50.0
    (:`OnSuccess`
      (`KismetSystemLibrary.PrintString` "Players Last Know Location"))
    (:`OnFail`
      _))
  (set `self.Chaseing Player` false))

(event `self.PawnSensing.OnSeePawn`
  (params (Pawn :type "Pawn Object Reference"))
  (`self.Get Player`))

(event `self.Sphere.OnComponentBeginOverlap`
  (params (OverlappedComponent :type "PrimitiveComponent Object Reference") (OtherActor :type "Actor Object Reference") (OtherComp :type "PrimitiveComponent Object Reference") (OtherBodyIndex :type Integer) (bFromSweep :type Boolean) (SweepResult :type "HitResult Structure (by ref)"))
  (bind _asbp_devvy (cast `/Game/Blueprints/BP_Devvy` OtherActor))
  (if (not (`self.IsStunned`))
    (`SceneComponent.K2_SetWorldTransform` (`Actor.RootComponent` _asbp_devvy) (`self.New Transform`) false false)))

(fn `Chase Player`)

(fn `UserConstructionScript`)