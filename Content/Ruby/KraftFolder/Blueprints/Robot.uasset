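; Robot companion actor that follows the player character, BP_Devvy, with a looping hover bob.
; On BeginPlay it looks up Devvy and the Robot by class and attaches the Robot to Devvy with relative rules.
; A restarting timeline adds bob offsets and sets Z around a fixed world height.
; Tick also sets the Robot's location, with sweep, to Devvy's position plus RobotLocationRef, which this graph never assigns.
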(event `self.ReceiveBeginPlay`
  (bind (_returnvalue_x _returnvalue_y) (`KismetMathLibrary.BreakVector` (`self.K2_GetActorLocation` (`self.RobotRef`))))
  (bind _returnvalue_x_2 (`KismetMathLibrary.BreakVector` (`self.K2_GetActorLocation` (`self.RobotRef`))))
  (`|ExecutionSequence`
    (:`then_0`
      ;[0 0.2566 1] Getting a reference for the player
      (bind _asbp_devvy (castclass `/Game/Blueprints/BP_Devvy` "/Game/Blueprints/BP_Devvy.BP_Devvy_C"))
      (bind _returnvalue (`GameplayStatics.GetActorOfClass` _asbp_devvy))
      (bind _output_get (set `self.PlayerRef` _returnvalue))
      ;[0.25 1 0.2249] Getting reference for robot
      (bind _asrobot (castclass `/Game/Ruby/KraftFolder/Blueprints/Robot` "Robot_C"))
      (bind _returnvalue_2 (`GameplayStatics.GetActorOfClass` _asrobot))
      (bind _output_get_2 (set `self.RobotRef` _returnvalue_2))
      (`self.K2_AttachToActor` _output_get_2 _output_get "None" "KeepRelative" "KeepRelative" "KeepRelative" true) ; Attaching Robot to Devvy. Ensures Robot is looking in correct direction.
      ;[0.25 1 0.2249] Robot bob animation. Only affects Z value.
      (bind (_direction _robotbob) (`Timeline|Timeline` :!label _label)
        (:`Update`
          (`self.K2_SetActorLocation` (`self.RobotRef`) (`KismetMathLibrary.MakeVector` (+ (.x _robotbob) _returnvalue_x_2) (+ (.y _robotbob) _returnvalue_y) (+ (.z _robotbob) 200.0)) false false))
        (:`Finished`
          (`KismetSystemLibrary.Delay` 0.01)
          (goto _label :!via `PlayFromStart`))))))

(event `self.ReceiveTick`
  (params (DeltaSeconds :type "Float (single-precision)"))
  ;[0.25 1 0.2249] Updates Robot location relative to Devvy (X, Y)  location.
  (bind _output_get (set `self.playerLocationRef` (`self.K2_GetActorLocation` (`self.PlayerRef`))))
  (`self.K2_SetActorLocation` (`self.RobotRef`) (+ _output_get (`self.robotLocationRef`)) true false))

(fn `UserConstructionScript`)