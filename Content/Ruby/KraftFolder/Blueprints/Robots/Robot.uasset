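; Companion robot actor that follows the player, Devvy, once HasRobot is set by Devvy overlapping its collision sphere.
; Tick places it at Devvy's location plus a stored offset, with sweep, and matches Devvy's camera rotation.
; BeginPlay caches player and robot references, and only if HasRobot is already true attaches the robot and starts a looping timeline bob.
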(event `self.ReceiveBeginPlay`
  (bind (_returnvalue_x _returnvalue_y _returnvalue_z) (`KismetMathLibrary.BreakVector` (`self.K2_GetActorLocation` (`self.RobotRef`))))
  (bind _returnvalue_x_2 (`KismetMathLibrary.BreakVector` (`self.K2_GetActorLocation` (`self.RobotRef`))))
  (bind (_returnvalue_x_3 _returnvalue_y_2) (`KismetMathLibrary.BreakVector` (`self.K2_GetActorLocation` (`self.RobotRef`))))
  ;[0 0.2566 1] Getting a reference for the player
  (bind _asbp_devvy (castclass `/Game/Blueprints/BP_Devvy` "/Game/Blueprints/BP_Devvy.BP_Devvy_C"))
  (bind _returnvalue (`GameplayStatics.GetActorOfClass` _asbp_devvy))
  (bind _output_get (set `self.PlayerRef` _returnvalue))
  ;[0.25 1 0.2249] Getting reference for robot
  (bind _asrobot (castclass `/Game/Ruby/KraftFolder/Blueprints/Robots/Robot` "Robot_C"))
  (bind _returnvalue_2 (`GameplayStatics.GetActorOfClass` _asrobot))
  (bind _output_get_2 (set `self.RobotRef` _returnvalue_2))
  (if (`self.hasRobot?`)
    (`self.K2_AttachToActor` _output_get_2 _output_get "None" "KeepRelative" "KeepRelative" "KeepRelative" true) ; Attaches Robot to Devvy. Keep location and rotation relative.
    ;[0.25 1 0.2249] Robot bob animation. Only affects Z value.
    (bind (_direction _robotbob) (`Timeline|Timeline` :!label _label)
      (:`Update`
        (`self.K2_SetActorLocation` (`self.RobotRef`) (`KismetMathLibrary.MakeVector` (+ (.x _robotbob) _returnvalue_x_2) (+ (.y _robotbob) _returnvalue_y_2) (+ (.z _robotbob) _returnvalue_z)) false false))
      (:`Finished`
        (`KismetSystemLibrary.Delay` 0.01)
        (goto _label :!via `PlayFromStart`)))))

(event `self.ReceiveTick`
  (params (DeltaSeconds :type "Float (single-precision)"))
  (if (`self.hasRobot?`)
    ;[0.25 1 0.2249] Updates Robot location relative to Devvy (X, Y, Z)  location.
    (bind _output_get (set `self.playerLocationRef` (`self.K2_GetActorLocation` (`self.PlayerRef`))))
    (`self.K2_SetActorLocation` (`self.RobotRef`) (+ _output_get (`self.robotLocationRef`)) true false)
    ;[0.25 1 0.2249] Updates Robot rotation relative to Devvy camera world rotation.
    (bind _output_get_2 (set `self.playerCamRotRef` (`SceneComponent.K2_GetComponentRotation` (`/Game/Blueprints/BP_Devvy.Camera` (`self.PlayerRef`)))))
    (`self.K2_SetActorRotation` (`self.RobotRef`) _output_get_2 false)))

(event `self.CollisionSphere.OnComponentBeginOverlap`
  (params (OverlappedComponent :type "PrimitiveComponent Object Reference") (OtherActor :type "Actor Object Reference") (OtherComp :type "PrimitiveComponent Object Reference") (OtherBodyIndex :type Integer) (bFromSweep :type Boolean) (SweepResult :type "HitResult Structure (by ref)"))
  (cast `/Game/Blueprints/BP_Devvy` OtherActor)
  (set `self.hasRobot?` true))

(fn `UserConstructionScript`)