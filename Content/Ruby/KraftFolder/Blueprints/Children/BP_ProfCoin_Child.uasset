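; Child Blueprint, apparently of a ProfCoin parent, that animates a coin actor through a timeline.
; BeginPlay calls the parent, then plays the CoinMotion timeline, which moves and rotates the actor on each update.
; The timeline's Z location and yaw are added to the actor's current values, so both accumulate per update, while roll and pitch are set directly.
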(event `self.ReceiveBeginPlay`
  (bind (_returnvalue_x _returnvalue_y _returnvalue_z) (`KismetMathLibrary.BreakVector` (`self.K2_GetActorLocation`)))
  (bind (_returnvalue_roll _returnvalue_pitch _returnvalue_yaw) (`KismetMathLibrary.BreakRotator` (`self.K2_GetActorRotation`)))
  (`parent.ReceiveBeginPlay`)
  (bind (_direction _location _rotation) (`Timeline|Coin Motion`)
    (:`Update`
      (`self.K2_SetActorLocationAndRotation` (`KismetMathLibrary.MakeVector` _returnvalue_x _returnvalue_y (+ _returnvalue_z (.z _location))) (`KismetMathLibrary.MakeRotator` (.x _rotation) (.y _rotation) (+ (.z _rotation) _returnvalue_yaw))))))

(fn `UserConstructionScript`
  (`parent.UserConstructionScript`))