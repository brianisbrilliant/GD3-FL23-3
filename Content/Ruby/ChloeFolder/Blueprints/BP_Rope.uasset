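; BP_Rope is a swingable rope actor that players grab on contact, with its CableEnd height set by Length at construction.
; Capsule overlap asks the other actor if it is a player and passes it the rope, gated by a DoOnce that resets on end overlap.
; AddSwingingForce pushes CableEnd as scaled acceleration, only while the end hangs far enough below the actor origin.
; A velocity-limiting branch is left unconnected.
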(event `self.Capsule.OnComponentBeginOverlap`
  (params (OverlappedComponent :type "PrimitiveComponent Object Reference") (OtherActor :type "Actor Object Reference") (OtherComp :type "PrimitiveComponent Object Reference") (OtherBodyIndex :type Integer) (bFromSweep :type Boolean) (SweepResult :type "HitResult Structure (by ref)"))
  (`/Engine/EditorBlueprintResources/StandardMacros.DoOnce` false :!label _label
    (:`Completed`
      (bind _yes_no (message `/Game/Ruby/ChloeFolder/Blueprints/BPI_Player.isPlayer` OtherActor))
      (if _yes_no
        (message `/Game/Ruby/ChloeFolder/Blueprints/BPI_Player.GrabRope` OtherActor self)
        (else
          (`KismetSystemLibrary.PrintString` "This is not a player"))))))

(event `self.Capsule.OnComponentEndOverlap`
  (params (OverlappedComponent :type "PrimitiveComponent Object Reference") (OtherActor :type "Actor Object Reference") (OtherComp :type "PrimitiveComponent Object Reference") (OtherBodyIndex :type Integer))
  (goto _label :!via `Reset`))

(event `AddSwingingForce`
  (params (SwingForce :type "Vector Structure"))
  (bind (_returnvalue_x _returnvalue_y _returnvalue_z) (`KismetMathLibrary.BreakVector` (`self.K2_GetActorLocation`)))
  (bind (_returnvalue_x_2 _returnvalue_y_2 _returnvalue_z_2) (`KismetMathLibrary.BreakVector` (`SceneComponent.K2_GetComponentLocation` (`self.CableEnd`))))
  (if (not (< (- _returnvalue_z _returnvalue_z_2) 350.0))
    (`PrimitiveComponent.AddForce` (`self.CableEnd`) (* SwingForce (500.0 500.0 500.0)) "None" true)))

(event `self.ReceiveTick`
  (params (DeltaSeconds :type "Float (single-precision)")))

(fn `UserConstructionScript`
  (`SceneComponent.K2_SetRelativeLocation` (`self.CableEnd`) (`KismetMathLibrary.MakeVector` 0.0 0.0 (`KismetMathLibrary.Conv_IntToDouble` (`self.Length`))) false false))