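; BP_Trigger_NextLevel is a gated level exit that sends the player on to ChloeLevel.
; Its Trigger event sets an Open flag and removes the fence mesh by disabling its collision and hiding it.
; When a BP_Jumper overlaps the Collision component while Open is set, it opens the next level by object reference.
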(event `self.Trigger`
  (bind _sm_prop_fence_01 (`self.SM_Prop_Fence_01`))
  (set `self.Open` true)
  (`PrimitiveComponent.SetCollisionEnabled` _sm_prop_fence_01 "NoCollision")
  (`SceneComponent.SetVisibility` _sm_prop_fence_01 false false))

(event `self.collision.OnComponentBeginOverlap`
  (params (OverlappedComponent :type "PrimitiveComponent Object Reference") (OtherActor :type "Actor Object Reference") (OtherComp :type "PrimitiveComponent Object Reference") (OtherBodyIndex :type Integer) (bFromSweep :type Boolean) (SweepResult :type "HitResult Structure (by ref)"))
  (cast `/Game/Ruby/TylersFolder/BP_Jumper` OtherActor)
  (if (`self.Open`)
    (`GameplayStatics.OpenLevelBySoftObjectPtr` "/Game/Ruby/ChloeFolder/Level/ChloeLevel.ChloeLevel")))

(fn `UserConstructionScript`
  (`parent.UserConstructionScript`))