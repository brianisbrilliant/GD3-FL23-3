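; BP_Prism is an interactable prism that sends the BP_Robot_Logan robot flying to it.
; A box overlap enables input while the player character is inside and disables it on exit.
; A left click then calls FlyToLocation on the robot, unless it already has a location specified, passing the RobotLocation component's position and the prism as target.
; The construction script applies a configurable world rotation to the prism mesh.
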(event `self.Box.OnComponentBeginOverlap`
  (params (OverlappedComponent :type "PrimitiveComponent Object Reference") (OtherActor :type "Actor Object Reference") (OtherComp :type "PrimitiveComponent Object Reference") (OtherBodyIndex :type Integer) (bFromSweep :type Boolean) (SweepResult :type "HitResult Structure (by ref)"))
  (if (== OtherActor (`GameplayStatics.GetPlayerCharacter` 0))
    (`self.EnableInput` (`GameplayStatics.GetPlayerController` 0))))

(event `self.Box.OnComponentEndOverlap`
  (params (OverlappedComponent :type "PrimitiveComponent Object Reference") (OtherActor :type "Actor Object Reference") (OtherComp :type "PrimitiveComponent Object Reference") (OtherBodyIndex :type Integer))
  (if (== OtherActor (`GameplayStatics.GetPlayerCharacter` 0))
    (`self.DisableInput` (`GameplayStatics.GetPlayerController` 0))))

(event `Key|LeftMouseButton`
  (params (Key :type "Key Structure"))
  (:`Pressed`
    (bind _returnvalue (`GameplayStatics.GetActorOfClass` "/Game/Ruby/Logan/Blueprints/BP_Robot_Logan.BP_Robot_Logan_C"))
    (if (not (`/Game/Ruby/KraftFolder/Blueprints/Robots/Robot.LocationSpecified` _returnvalue))
      (`/Game/Ruby/KraftFolder/Blueprints/Robots/Robot.FlyToLocation` _returnvalue (`self.K2_GetActorLocation` _returnvalue) (`SceneComponent.K2_GetComponentLocation` (`self.RobotLocation`)) (`self.K2_GetActorLocation`) self))))

(fn `UserConstructionScript`
  (`SceneComponent.K2_SetWorldRotation` (`self.PrismMesh`) (`self.PrismRotation`) false false))