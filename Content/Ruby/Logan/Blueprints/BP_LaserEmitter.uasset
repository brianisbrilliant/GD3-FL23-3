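; Laser emitter actor that casts a beam from its arrow, bouncing it off mirrors and redirecting it through prisms to toggle sensors.
; CastLight loops complex line traces, identifying mirrors and prisms by hit-face material, activating a hit BP_Sensor or deactivating the stored one otherwise.
; At runtime, delayed Tick calls destroy and respawn a BP_LaserBeam per segment.
; EditorTick previews the path with debug traces only.
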(event `self.ReceiveTick`
  (params (DeltaSeconds :type "Float (single-precision)"))
  (bind _arrow (`self.Arrow`))
  (set `self.IsEditor` false)
  (set `self.LaserDebugType` "None")
  (`KismetSystemLibrary.Delay` 0.01)
  (`self.CastLight` (`SceneComponent.K2_GetComponentLocation` _arrow) (`SceneComponent.GetForwardVector` _arrow) (`self.CastDistance`) :!label _label))

(event `/Game/Ruby/Logan/Blueprints/BPI_EditorTick.EditorTick`
  (set `self.IsEditor` true)
  (set `self.LaserDebugType` "ForDuration")
  (goto _label))

(fn `CastLight`
  (params (CastOrigin :type "Vector Structure") (CastDirection :type "Vector Structure") (CastDistance :type "Float (double-precision)"))
  (locals (L_CastOrigin :type "Vector Structure") (L_CastDirection :type "Vector Structure") (L_CastDistance :type "Float (double-precision)") (L_Continue :type Boolean :default true) (L_BeamStart :type "Vector Structure") (L_BeamEnd :type "Vector Structure"))
  (bind _l_castorigin (`local.L_CastOrigin`))
  (bind _returnvalue (+ _l_castorigin (* (`local.L_CastDirection`) (`local.L_CastDistance`))))
  (set `local.L_CastOrigin` CastOrigin)
  (set `local.L_CastDirection` CastDirection)
  (set `local.L_CastDistance` CastDistance)
  (if (not (`self.IsEditor`))
    (for _array_element (`self.Beams`)
      (`self.K2_DestroyActor` _array_element))
    (`KismetArrayLibrary.Array_Clear` (`self.Beams`)))
  (while (`local.L_Continue`)
    (`|ExecutionSequence`
      (:`then_0`
        (bind (_outhit _returnvalue_2) (`KismetSystemLibrary.LineTraceSingle` :`Start` _l_castorigin :`End` _returnvalue :`TraceChannel` "TraceTypeQuery1" :`bTraceComplex` true :`DrawDebugType` (`self.LaserDebugType`) :`DrawTime` 0.1))
        (set `local.L_BeamStart` (`local.L_CastOrigin`))
        (if _returnvalue_2
          (bind (_bblockinghit _binitialoverlap _time _distance _location _impactpoint _normal _impactnormal _physmat _hitactor _hitcomponent _hitbonename _bonename _hititem _elementindex _faceindex) (`GameplayStatics.BreakHitResult` _outhit))
          (set `local.L_BeamEnd` _impactpoint)
          (bind (_sectionindex _returnvalue_3) (`PrimitiveComponent.GetMaterialFromCollisionFaceIndex` _hitcomponent _faceindex))
          (if (== _returnvalue_3 "/Game/Ruby/Logan/Material/M_Mirror.M_Mirror")
            (set `local.L_CastOrigin` _impactpoint)
            (set `local.L_CastDirection` (`KismetMathLibrary.MirrorVectorByNormal` (`local.L_CastDirection`) _impactnormal))
            (set `local.L_Continue` true)
            (elif (== _returnvalue_3 "/Game/Ruby/Logan/Material/M_Prism.M_Prism")
              (bind _asbp_prism (cast `/Game/Ruby/Logan/Blueprints/BP_Prism` _hitactor))
              (set `local.L_CastDirection` (`SceneComponent.GetForwardVector` (`/Game/Ruby/Logan/Blueprints/BP_Prism.Arrow` _asbp_prism)))
              (set `local.L_CastOrigin` (`SceneComponent.K2_GetComponentLocation` (`/Game/Ruby/Logan/Blueprints/BP_Prism.LaserSpawn` _asbp_prism)))
              (set `local.L_Continue` true)
              (else
                (bind _asbp_sensor (cast `/Game/Ruby/Logan/Blueprints/BP_Sensor` _hitactor)
                  (:`then`
                    (`/Game/Ruby/Logan/Blueprints/BPI_SetSensorState.ToggleState` _asbp_sensor true)
                    (set `self.ActivatedSensor` _asbp_sensor)
                    (set `local.L_Continue` false))
                  (:`CastFailed`
                    (set `local.L_Continue` false :!label _label)
                    (`/Engine/EditorBlueprintResources/StandardMacros.IsValid` (`self.ActivatedSensor`)
                      (:`Is Valid`
                        (`/Game/Ruby/Logan/Blueprints/BPI_SetSensorState.ToggleState` (`self.ActivatedSensor`) false))))))))
          (else
            (set `local.L_BeamEnd` _returnvalue)
            (goto _label))))
      (:`then_1`
        (if (not (`self.IsEditor`))
          (bind _returnvalue_4 (`|SpawnActorFromClass` "/Game/Ruby/Logan/Blueprints/BP_LaserBeam.BP_LaserBeam_C" (`KismetMathLibrary.MakeTransform` (0.0 0.0 0.0)) "Undefined" "MultiplyWithRoot" null null))
          (`/Game/Ruby/Logan/Blueprints/BP_LaserBeam.SetEnds` _returnvalue_4 (`local.L_BeamStart`) (`local.L_BeamEnd`))
          (`KismetArrayLibrary.Array_Add` (`self.Beams`) _returnvalue_4))))))

(fn `UserConstructionScript`
  (`AddComponent|NODE_AddChildActorComponent-0`))