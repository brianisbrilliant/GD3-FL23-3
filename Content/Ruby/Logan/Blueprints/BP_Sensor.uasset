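; BP_Sensor is a switch that fires its linked TriggerObject when a BP_Laser hits it or when ToggleState turns it on.
; Laser hits trigger immediately and destroy the laser, while activation cuts to CameraView for a few seconds and triggers after a short delay.
; When BP_Devvy is in range, it shows an info widget and enables input, so holding right mouse previews CameraView and highlights the linked object.
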(event `self.ReceiveBeginPlay`)

(event `self.Box.OnComponentBeginOverlap`
  (params (OverlappedComponent :type "PrimitiveComponent Object Reference") (OtherActor :type "Actor Object Reference") (OtherComp :type "PrimitiveComponent Object Reference") (OtherBodyIndex :type Integer) (bFromSweep :type Boolean) (SweepResult :type "HitResult Structure (by ref)"))
  (bind _triggerobject (`self.TriggerObject`))
  (cast `/Game/Ruby/Logan/Blueprints/BP_Laser` OtherActor)
  (`/Engine/EditorBlueprintResources/StandardMacros.IsValid` _triggerobject
    (:`Is Valid`
      (`/Game/Ruby/Logan/Blueprints/BP_TriggerObject.Trigger` _triggerobject)
      (`self.K2_DestroyActor` OtherActor))))

(event `Activate`
  (bind _triggerobject (`self.TriggerObject`))
  (`/Engine/EditorBlueprintResources/StandardMacros.IsValid` _triggerobject
    (:`Is Valid`
      (`self.ShowTriggeredObject`)
      (`KismetSystemLibrary.Delay` 1.0)
      (`/Game/Ruby/Logan/Blueprints/BP_TriggerObject.Trigger` _triggerobject))))

(event `/Game/Ruby/Logan/Blueprints/BPI_SetSensorState.ToggleState`
  (params (`On/Off` :type Boolean))
  (if (and (== `On/Off` true) (== (`self.IsActive`) false))
    (`self.Activate`))
  (set `self.IsActive` `On/Off`))

(event `self.Box1.OnComponentBeginOverlap`
  (params (OverlappedComponent :type "PrimitiveComponent Object Reference") (OtherActor :type "Actor Object Reference") (OtherComp :type "PrimitiveComponent Object Reference") (OtherBodyIndex :type Integer) (bFromSweep :type Boolean) (SweepResult :type "HitResult Structure (by ref)"))
  (cast `/Game/Blueprints/BP_Devvy` OtherActor)
  (`/Engine/EditorBlueprintResources/StandardMacros.DoOnce` false :!label _label
    (:`Completed`
      (`self.EnableInput` (`GameplayStatics.GetPlayerController` 0))
      (bind _returnvalue (`|CreateWidget` "/Game/Ruby/Logan/Blueprints/W_SensorInfo.W_SensorInfo_C"))
      (set `self.SpawnedInfoWidget` _returnvalue)
      (`UserWidget.AddToViewport` _returnvalue 0))))

(event `self.Box1.OnComponentEndOverlap`
  (params (OverlappedComponent :type "PrimitiveComponent Object Reference") (OtherActor :type "Actor Object Reference") (OtherComp :type "PrimitiveComponent Object Reference") (OtherBodyIndex :type Integer))
  (cast `/Game/Blueprints/BP_Devvy` OtherActor)
  (`self.DisableInput` (`GameplayStatics.GetPlayerController` 0))
  (`Widget.RemoveFromParent` (`self.SpawnedInfoWidget`))
  (goto _label :!via `Reset`))

(event `Key|RightMouseButton`
  (params (Key :type "Key Structure"))
  (:`Pressed`
    (`PlayerController.SetViewTargetWithBlend` (`GameplayStatics.GetPlayerController` 0) (`self.CameraView`) 0.0 "VTBlend_Linear" 0.0 false :!label _label_2)
    (`/Game/Ruby/Logan/Blueprints/BP_TriggerObject.HighlightTriggerObject` (`self.TriggerObject`)))
  (:`Released`
    (`PlayerController.SetViewTargetWithBlend` (`GameplayStatics.GetPlayerController` 0) (`GameplayStatics.GetPlayerCharacter` 0) 0.0 "VTBlend_Linear" 0.0 false :!label _label_3)
    (`/Game/Ruby/Logan/Blueprints/BP_TriggerObject.UnHighlightTriggerObject` (`self.TriggerObject`))))

(event `Key|RightMouseButton`
  (params (Key :type "Key Structure"))
  (:`Pressed`
    (goto _label_2))
  (:`Released`
    (goto _label_3)))

(event `ShowTriggeredObject`
  (`PlayerController.SetViewTargetWithBlend` (`GameplayStatics.GetPlayerController` 0) (`self.CameraView`) 0.0 "VTBlend_Linear" 0.0 false)
  (`KismetSystemLibrary.Delay` 4.0)
  (`PlayerController.SetViewTargetWithBlend` (`GameplayStatics.GetPlayerController` 0) (`GameplayStatics.GetPlayerCharacter` 0) 0.0 "VTBlend_Linear" 0.0 false))

(fn `UserConstructionScript`)