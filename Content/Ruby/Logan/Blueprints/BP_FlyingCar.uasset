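; BP_FlyingCar is an actor that flies in a straight, looping path.
; Its construction script sets the yaw from the Rotation variable.
; Each Tick moves it along its forward vector by Speed without sweeping or delta-time scaling, so its pace depends on frame rate.
; Once its distance from StartPos reaches MaxDistance, it jumps back to StartPos, which these graphs never assign.
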(event `self.ReceiveBeginPlay`)

(event `self.ReceiveTick`
  (params (DeltaSeconds :type "Float (single-precision)"))
  (`self.K2_SetActorLocation` (+ (* (`self.GetActorForwardVector`) (`self.Speed`)) (`self.K2_GetActorLocation`)))
  (if (>= (`KismetMathLibrary.Vector_Distance` (`self.K2_GetActorLocation`) (`self.StartPos`)) (`self.MaxDistance`))
    (`self.K2_SetActorLocation` (`self.StartPos`))))

(fn `UserConstructionScript`
  (`self.K2_SetActorRotation` (`KismetMathLibrary.MakeRotator` 0.0 0.0 (`self.Rotation`))))