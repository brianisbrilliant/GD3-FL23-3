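; BP_TriggerObject is a triggerable object with a blinking highlight, whose Trigger event currently only prints a debug greeting.
; The highlight component starts hidden, and the construction script sets its scale from HighlightScale.
; HighlightTriggerObject blinks it through a looped Delay toggle while the Highlighted flag stays set, ignoring repeat calls.
; UnHighlightTriggerObject clears the flag and hides the highlight.
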(event `self.ReceiveBeginPlay`
  (`SceneComponent.SetVisibility` (`self.Highlight`) false false))

(event `Trigger`
  (`KismetSystemLibrary.PrintString` "Hello"))

(event `HighlightTriggerObject`
  (if (== (`self.Highlighted`) false)
    (set `self.Highlighted` true)
    (`SceneComponent.SetVisibility` (`self.Highlight`) true false :!label _label)
    (`KismetSystemLibrary.Delay` 0.3)
    (`SceneComponent.SetVisibility` (`self.Highlight`) false false)
    (`KismetSystemLibrary.Delay` 0.3)
    (if (`self.Highlighted`)
      (goto _label))))

(event `UnHighlightTriggerObject`
  (set `self.Highlighted` false)
  (`SceneComponent.SetVisibility` (`self.Highlight`) false false))

(fn `UserConstructionScript`
  (`SceneComponent.SetRelativeScale3D` (`self.Highlight`) (`self.HighlightScale`)))