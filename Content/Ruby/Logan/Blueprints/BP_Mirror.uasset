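; BP_Mirror is a rotatable mirror that redirects BP_Laser actors in what appears to be a light-beam puzzle.
; Player overlap with Box enables input, letting R cycle Cube through preset Rotations.
; Box1 replaces incoming lasers with a new one, aimed at NextMirror when the rotation index is correct, otherwise along Cube's rotation.
; Cube destroys other lasers, while collision toggling and a SpawnedLaser check guard against self-triggering.
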(event `self.Box1.OnComponentBeginOverlap`
  (params (OverlappedComponent :type "PrimitiveComponent Object Reference") (OtherActor :type "Actor Object Reference") (OtherComp :type "PrimitiveComponent Object Reference") (OtherBodyIndex :type Integer) (bFromSweep :type Boolean) (SweepResult :type "HitResult Structure (by ref)"))
  (bind _returnvalue_location (`KismetMathLibrary.BreakTransform` (`self.GetTransform` OtherActor)))
  (bind _asbp_laser (cast `/Game/Ruby/Logan/Blueprints/BP_Laser` OtherActor))
  (if (not (== _asbp_laser (`self.SpawnedLaser`)))
    (set `self.LaserSpawnPoint` _returnvalue_location)
    (`self.K2_DestroyActor` _asbp_laser)
    (`self.SetActorEnableCollision` false)
    (if (and (`KismetSystemLibrary.IsValid` (`self.NextMirror`)) (== (`self.CorrectRotationIndex`) (`self.CurrentRotationIndex`)))
      (bind _returnvalue (`|SpawnActorFromClass` "/Game/Ruby/Logan/Blueprints/BP_Laser.BP_Laser_C" (`KismetMathLibrary.MakeTransform` (`self.LaserSpawnPoint`) (`KismetMathLibrary.FindLookAtRotation` (`SceneComponent.K2_GetComponentLocation` (`self.Plane`)) (`SceneComponent.K2_GetComponentLocation` (`/Game/Ruby/Logan/Blueprints/BP_Mirror.Plane` (`self.NextMirror`)))) (0.075408 0.075408 0.075408)) "Undefined" "MultiplyWithRoot" null null))
      (set `self.SpawnedLaser` _returnvalue)
      (else
        (bind _returnvalue_2 (`|SpawnActorFromClass` "/Game/Ruby/Logan/Blueprints/BP_Laser.BP_Laser_C" (`KismetMathLibrary.MakeTransform` (`self.LaserSpawnPoint`) (`SceneComponent.K2_GetComponentRotation` (`self.Cube`)) (0.075408 0.075408 0.075408)) "Undefined" "MultiplyWithRoot" null null))
        (set `self.SpawnedLaser` _returnvalue_2)))
    (`self.SetActorEnableCollision` true)))

(event `self.Box.OnComponentBeginOverlap`
  (params (OverlappedComponent :type "PrimitiveComponent Object Reference") (OtherActor :type "Actor Object Reference") (OtherComp :type "PrimitiveComponent Object Reference") (OtherBodyIndex :type Integer) (bFromSweep :type Boolean) (SweepResult :type "HitResult Structure (by ref)"))
  (if (== OtherActor (`GameplayStatics.GetPlayerCharacter` 0))
    (`self.EnableInput` (`GameplayStatics.GetPlayerController` 0))))

(event `Key|R`
  (params (Key :type "Key Structure"))
  (:`Pressed`
    (`/Engine/EditorBlueprintResources/StandardMacros.DoOnce` false :!label _label
      (:`Completed`
        (if (< (`self.CurrentRotationIndex`) (- (`KismetArrayLibrary.Array_Length` (`self.Rotations`)) 1))
          (`/Engine/EditorBlueprintResources/StandardMacros.IncrementInt` (`self.CurrentRotationIndex`)
            (:`  `
              _))
          (else
            (set `self.CurrentRotationIndex` 0)))
        (`SceneComponent.K2_SetWorldRotation` (`self.Cube`) (`|GetArrayItem` (`self.Rotations`) (`self.CurrentRotationIndex`)) false false))))
  (:`Released`
    (goto _label :!via `Reset`)))

(event `self.Cube.OnComponentBeginOverlap`
  (params (OverlappedComponent :type "PrimitiveComponent Object Reference") (OtherActor :type "Actor Object Reference") (OtherComp :type "PrimitiveComponent Object Reference") (OtherBodyIndex :type Integer) (bFromSweep :type Boolean) (SweepResult :type "HitResult Structure (by ref)"))
  (bind _asbp_laser (cast `/Game/Ruby/Logan/Blueprints/BP_Laser` OtherActor))
  (if (!= _asbp_laser (`self.SpawnedLaser`))
    (`self.K2_DestroyActor` _asbp_laser)))

(fn `UserConstructionScript`)