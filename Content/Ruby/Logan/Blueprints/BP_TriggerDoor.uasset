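; Door actor that slides its Cube mesh vertically when its Trigger event fires.
; BeginPlay caches the Cube's relative location as Origin, and Trigger plays a Timeline whose track is added to Origin's Z on each update, without sweep.
; It has no closing or reverse logic, and its overlap and Tick events are disabled.
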(event `self.ReceiveBeginPlay`
  (`parent.ReceiveBeginPlay`)
  (set `self.Origin` (`SceneComponent.RelativeLocation` (`self.Cube`))))

(event `self.Trigger`
  (bind (_origin_x _origin_y _origin_z) (`KismetMathLibrary.BreakVector` (`self.Origin`)))
  (bind (_direction _newtrack_0) (`Timeline|Timeline`)
    (:`Update`
      (`SceneComponent.K2_SetRelativeLocation` (`self.Cube`) (`KismetMathLibrary.MakeVector` _origin_x _origin_y (+ _origin_z _newtrack_0)) false false))))

(fn `UserConstructionScript`
  (`parent.UserConstructionScript`))