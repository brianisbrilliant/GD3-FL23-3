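; BP_RotatorPad is a rotating pad that turns up to four colour-slot actors, attached at BeginPlay, around its Rotator.
; Trigger runs a timeline that yaws the Rotator by RotationAngle, clearing Unlocked until it finishes.
; With ButtonActivated, the button is visible, and BP_Devvy overlapping its box enables input and an info widget.
; Right mouse or gamepad trigger presses it, calling Trigger when unlocked; Tick colours it green or red.
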(event `self.ReceiveBeginPlay`
  (`SceneComponent.SetVisibility` (`self.Highlight`) false false)
  (`|ExecutionSequence`
    (:`then_0`
      (`/Engine/EditorBlueprintResources/StandardMacros.IsValid` (`self.RedSlotActor`)
        (:`Is Valid`
          (`self.K2_AttachToComponent` (`self.RedSlotActor`) (`self.Rotator`) "None" "KeepWorld" "KeepWorld" "KeepWorld" true))))
    (:`then_1`
      (`/Engine/EditorBlueprintResources/StandardMacros.IsValid` (`self.BlueSlotActor`)
        (:`Is Valid`
          (`self.K2_AttachToComponent` (`self.BlueSlotActor`) (`self.Rotator`) "None" "KeepWorld" "KeepWorld" "KeepWorld" true))))
    (:`then_2`
      (`/Engine/EditorBlueprintResources/StandardMacros.IsValid` (`self.GreenSlotActor`)
        (:`Is Valid`
          (`self.K2_AttachToComponent` (`self.GreenSlotActor`) (`self.Rotator`) "None" "KeepWorld" "KeepWorld" "KeepWorld" true))))
    (:`then_3`
      (`/Engine/EditorBlueprintResources/StandardMacros.IsValid` (`self.YellowSlotActor`)
        (:`Is Valid`
          (`self.K2_AttachToComponent` (`self.YellowSlotActor`) (`self.Rotator`) "None" "KeepWorld" "KeepWorld" "KeepWorld" true))))))

(event `self.Trigger`
  (`GameplayStatics.PlaySoundAtLocation` "/Game/Ruby/Logan/RotateSound.RotateSound" (0.0 0.0 0.0) (struct) 1.0 1.0 0.0 null null null null)
  ;[1 1 1] Rotate Lilylaunchpads
  (set `self.Unlocked` false)
  (set `self.OriginRotation` (`SceneComponent.K2_GetComponentRotation` (`self.Rotator`)))
  (bind (_direction _newtrack_0) (`Timeline|Timeline` :!via `PlayFromStart`)
    (:`Update`
      (`SceneComponent.K2_SetWorldRotation` (`self.Rotator`) (`KismetMathLibrary.MakeRotator` (.roll (`self.OriginRotation`)) (.pitch (`self.OriginRotation`)) (+ (.yaw (`self.OriginRotation`)) (.yaw (`KismetMathLibrary.MakeRotator` 0.0 0.0 (* _newtrack_0 (`self.RotationAngle`)))))) false false))
    (:`Finished`
      (set `self.Unlocked` true))))

(event `self.ButtonBox.OnComponentBeginOverlap`
  (params (OverlappedComponent :type "PrimitiveComponent Object Reference") (OtherActor :type "Actor Object Reference") (OtherComp :type "PrimitiveComponent Object Reference") (OtherBodyIndex :type Integer) (bFromSweep :type Boolean) (SweepResult :type "HitResult Structure (by ref)"))
  (cast `/Game/Blueprints/BP_Devvy` OtherActor)
  (if (`self.ButtonActivated`)
    (`/Engine/EditorBlueprintResources/StandardMacros.DoOnce` false :!label _label
      (:`Completed`
        (`self.EnableInput` (`GameplayStatics.GetPlayerController` 0))
        (bind _returnvalue (`|CreateWidget` "/Game/Ruby/Logan/Blueprints/W_ButtonInfo.W_ButtonInfo_C"))
        (set `self.SpawnedInfoWidget` _returnvalue)
        (`UserWidget.AddToViewport` _returnvalue 0)))))

(event `self.ButtonBox.OnComponentEndOverlap`
  (params (OverlappedComponent :type "PrimitiveComponent Object Reference") (OtherActor :type "Actor Object Reference") (OtherComp :type "PrimitiveComponent Object Reference") (OtherBodyIndex :type Integer))
  (if (`self.ButtonActivated`)
    (cast `/Game/Blueprints/BP_Devvy` OtherActor)
    (`self.DisableInput` (`GameplayStatics.GetPlayerController` 0))
    (`Widget.RemoveFromParent` (`self.SpawnedInfoWidget`))
    (goto _label :!via `Reset`)))

(event `Key|RightMouseButton`
  (params (Key :type "Key Structure"))
  (bind _button (`self.Button`))
  (bind _buttonactivated (`self.ButtonActivated`))
  (:`Pressed`
    (if _buttonactivated :!label _label_2
      (`SceneComponent.K2_AddLocalOffset` _button (0.0 0.0 -10.0) false false)
      (if (`self.Unlocked`)
        (`self.Trigger`))))
  (:`Released`
    (if _buttonactivated :!label _label_3
      (`SceneComponent.K2_AddLocalOffset` _button (0.0 0.0 10.0) false false))))

(event `Key|Gamepad_RightTrigger`
  (params (Key :type "Key Structure"))
  (:`Pressed`
    (goto _label_2))
  (:`Released`
    (goto _label_3)))

(event `self.ReceiveTick`
  (params (DeltaSeconds :type "Float (single-precision)"))
  (bind _button (`self.Button`))
  (if (`self.Unlocked`)
    (`PrimitiveComponent.SetMaterial` _button 0 "/Game/Ruby/Logan/Material/M_Green.M_Green")
    (else
      (`PrimitiveComponent.SetMaterial` _button 0 "/Game/Ruby/Logan/Material/M_Red.M_Red"))))

(fn `UserConstructionScript`
  (bind _buttonpost (`self.ButtonPost`))
  (`SceneComponent.SetRelativeScale3D` (`self.Highlight`) (`self.HighlightScale`))
  (if (`self.ButtonActivated`)
    (`SceneComponent.SetVisibility` _buttonpost true false)
    (`SceneComponent.SetVisibility` (`self.ButtonBox`) true false)
    (`SceneComponent.SetVisibility` (`self.Button`) true false)
    (else
      (`SceneComponent.SetVisibility` _buttonpost false false)
      (`SceneComponent.SetVisibility` (`self.ButtonBox`) false false)
      (`SceneComponent.SetVisibility` (`self.Button`) false false))))