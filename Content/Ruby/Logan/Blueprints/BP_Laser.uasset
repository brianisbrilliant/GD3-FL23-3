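; BP_Laser is a projectile actor that travels in a straight line and destroys itself after a Lifespan delay.
; Each Tick teleports it along its forward vector by Speed without sweep or delta-time scaling, so its velocity depends on frame rate.
; Its hit and overlap events are empty, and a disconnected BP_Mirror check that would destroy it on non-mirror actors never runs.
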(event `self.ReceiveBeginPlay`
  (`KismetSystemLibrary.Delay` (`self.Lifespan`))
  (`self.K2_DestroyActor`))

(event `self.Cylinder.OnComponentHit`
  (params (HitComponent :type "PrimitiveComponent Object Reference") (OtherActor :type "Actor Object Reference") (OtherComp :type "PrimitiveComponent Object Reference") (NormalImpulse :type "Vector Structure") (Hit :type "HitResult Structure (by ref)")))

(event `self.ReceiveActorBeginOverlap`
  (params (OtherActor :type "Actor Object Reference")))

(event `self.ReceiveTick`
  (params (DeltaSeconds :type "Float (single-precision)"))
  (`self.K2_SetActorLocation` (+ (`self.K2_GetActorLocation`) (* (`self.GetActorForwardVector`) (`self.Speed`))) false true))

(fn `UserConstructionScript`)