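; BP_DestructibleObject_Child is a destructible object Blueprint that explodes when its Destroy event fires.
; Destroy plays a non-spatialized explosion cue, spawns BP_Explosion at the actor's transform, then removes the actor.
; The construction script defers to the parent, and the BeginPlay, overlap and Tick stubs are disabled, so this graph adds only the destruction response.
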(event `self.Destroy`
  (`GameplayStatics.PlaySound2D` "/Game/Ruby/JohnFolder/John_Content/StarterContent/Audio/Explosion_Cue.Explosion_Cue" 1.0 1.0 0.0 null null)
  (`|SpawnActorFromClass` "/Game/Ruby/JohnFolder/John_Blueprints/BP_Explosion.BP_Explosion_C" (`self.GetTransform`) "Undefined" "MultiplyWithRoot" null null)
  (`self.K2_DestroyActor`))

(fn `UserConstructionScript`
  (`parent.UserConstructionScript`))