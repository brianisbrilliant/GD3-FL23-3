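; BP_Police_12 is a police vehicle actor that travels along a spline path in the level once play begins.
; On BeginPlay it finds the BP_Spline_12 actor and starts a timeline with play rate set to the inverse of TimeToComplete.
; Each update maps the timeline's Move track to distance along the spline, then sets the actor's world location and rotation from that point.
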(event `self.ReceiveBeginPlay`
  (bind _returnvalue (`GameplayStatics.GetActorOfClass` "/Game/Ruby/JohnFolder/John_Blueprints/Vehicles/BP_Spline_12.BP_Spline_12_C"))
  (set `self.Spline 12` _returnvalue)
  (`self.Move Object`))

(event `Move Object`
  (bind _spline (`/Game/Ruby/JohnFolder/John_Blueprints/Vehicles/BP_Spline_12.Spline` (`self.Spline 12`)))
  (`TimelineComponent.SetPlayRate` (`self.Timeline`) (/ 1.0 (`self.Time to Complete`)))
  (bind (_direction _move) (`Timeline|Timeline`)
    (:`Update`
      (bind _returnvalue (`KismetMathLibrary.Lerp` 0.0 (`SplineComponent.GetSplineLength` (`/Game/Ruby/JohnFolder/John_Blueprints/Vehicles/BP_Spline_12.Spline` (`self.Spline 12`))) _move))
      (`self.K2_SetActorTransform` (`KismetMathLibrary.MakeTransform` (`SplineComponent.GetLocationAtDistanceAlongSpline` _spline _returnvalue "World") (`SplineComponent.GetRotationAtDistanceAlongSpline` _spline _returnvalue "World"))))))

(fn `UserConstructionScript`)