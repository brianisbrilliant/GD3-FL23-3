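; BP_Police is a police vehicle actor that travels along a spline path in the level.
; On BeginPlay it finds a BP_Spline actor and plays a timeline whose rate is set from TimeToComplete.
; Each timeline update maps the Move value to a distance along the spline and sets the actor's world location and rotation to match that point.
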(event `self.ReceiveBeginPlay`
  (bind _returnvalue (`GameplayStatics.GetActorOfClass` "/Game/Ruby/JohnFolder/John_Blueprints/Vehicles/BP_Spline.BP_Spline_C"))
  (set `self.Spline Ref` _returnvalue)
  (`self.Move Object`))

(event `Move Object`
  (bind _spline (`/Game/Ruby/JohnFolder/John_Blueprints/Vehicles/BP_Spline.Spline` (`self.Spline Ref`)))
  (`TimelineComponent.SetPlayRate` (`self.Timeline`) (/ 1.0 (`self.Time to Complete`)))
  (bind (_direction _move) (`Timeline|Timeline`)
    (:`Update`
      (bind _returnvalue (`KismetMathLibrary.Lerp` 0.0 (`SplineComponent.GetSplineLength` (`/Game/Ruby/JohnFolder/John_Blueprints/Vehicles/BP_Spline.Spline` (`self.Spline Ref`))) _move))
      (`self.K2_SetActorTransform` (`KismetMathLibrary.MakeTransform` (`SplineComponent.GetLocationAtDistanceAlongSpline` _spline _returnvalue "World") (`SplineComponent.GetRotationAtDistanceAlongSpline` _spline _returnvalue "World"))))))

(fn `UserConstructionScript`)