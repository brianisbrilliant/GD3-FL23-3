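; BP_Police_18 is a police vehicle actor that moves itself along a spline path from BeginPlay.
; It finds the BP_Spline_18 actor in the level and runs a timeline with its play rate scaled by TimeToComplete.
; Each timeline update maps the Move alpha to a distance along the spline and sets the actor's world location and rotation to match.
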(event `self.ReceiveBeginPlay`
  (bind _returnvalue (`GameplayStatics.GetActorOfClass` "/Game/Ruby/JohnFolder/John_Blueprints/Vehicles/BP_Spline_18.BP_Spline_18_C"))
  (set `self.Spline 18` _returnvalue)
  (`self.Move Object`))

(event `Move Object`
  (bind _spline (`/Game/Ruby/JohnFolder/John_Blueprints/Vehicles/BP_Spline_18.Spline` (`self.Spline 18`)))
  (`TimelineComponent.SetPlayRate` (`self.Timeline`) (/ 1.0 (`self.Time to Complete`)))
  (bind (_direction _move) (`Timeline|Timeline`)
    (:`Update`
      (bind _returnvalue (`KismetMathLibrary.Lerp` 0.0 (`SplineComponent.GetSplineLength` (`/Game/Ruby/JohnFolder/John_Blueprints/Vehicles/BP_Spline_18.Spline` (`self.Spline 18`))) _move))
      (`self.K2_SetActorTransform` (`KismetMathLibrary.MakeTransform` (`SplineComponent.GetLocationAtDistanceAlongSpline` _spline _returnvalue "World") (`SplineComponent.GetRotationAtDistanceAlongSpline` _spline _returnvalue "World"))))))

(fn `UserConstructionScript`)