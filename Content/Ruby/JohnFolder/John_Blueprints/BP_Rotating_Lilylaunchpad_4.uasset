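; Rotating lily launchpad actor that endlessly alternates between two orientations once triggered by an overlap with its Box.
; The overlap runs through a FlipFlop with only A wired, so every other overlap calls Rotate.
; Rotate loops two near-instant MoveComponentTo snaps on the root, each followed by a two-second delay.
; Rotate2 enters the loop at the second orientation, but its only call is disconnected.
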(event `Rotate`
  ;[1 1 1] Rotate Lilylaunchpads
  (`KismetSystemLibrary.MoveComponentTo` (`self.DefaultSceneRoot`) (`self.K2_GetActorLocation`) (struct :`Yaw` -90.0) false false 0.01 :!label _label)
  (`KismetSystemLibrary.Delay` 2.0)
  (`KismetSystemLibrary.MoveComponentTo` (`self.DefaultSceneRoot`) (`self.K2_GetActorLocation`) (struct :`Yaw` 360.0) false false 0.01 :!label _label_2)
  (`KismetSystemLibrary.Delay` 2.0)
  (goto _label))

(event `Rotate 2`
  ;[1 1 1] Rotate Lilylaunchpads
  (goto _label_2))

(event `self.Box.OnComponentBeginOverlap`
  (params (OverlappedComponent :type "PrimitiveComponent Object Reference") (OtherActor :type "Actor Object Reference") (OtherComp :type "PrimitiveComponent Object Reference") (OtherBodyIndex :type Integer) (bFromSweep :type Boolean) (SweepResult :type "HitResult Structure (by ref)"))
  ;[1 1 1] Rotate Lilylaunchpads
  (`/Engine/EditorBlueprintResources/StandardMacros.FlipFlop`
    (:`A`
      (`self.Rotate`))))

(fn `UserConstructionScript`)