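; Lily launchpad actor that snaps between two fixed orientations, a quarter turn apart, as things overlap its Box.
; Begin overlap fires a DoOnce that end overlap re-arms, and a FlipFlop alternates between the Rotate and Rotate2 events.
; Each event uses MoveComponentTo on the root for a near-instant turn, passing the current actor location as the target position.
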(event `Rotate`
  ;[1 1 1] Rotate Lilylaunchpads
  (`KismetSystemLibrary.MoveComponentTo` (`self.DefaultSceneRoot`) (`self.K2_GetActorLocation`) (struct :`Yaw` 270.0) false false 0.01))

(event `Rotate 2`
  ;[1 1 1] Rotate Lilylaunchpads
  (`KismetSystemLibrary.MoveComponentTo` (`self.DefaultSceneRoot`) (`self.K2_GetActorLocation`) (struct :`Yaw` 360.0) false false 0.01))

(event `self.Box.OnComponentEndOverlap`
  (params (OverlappedComponent :type "PrimitiveComponent Object Reference") (OtherActor :type "Actor Object Reference") (OtherComp :type "PrimitiveComponent Object Reference") (OtherBodyIndex :type Integer))
  (goto _label :!via `Reset`))

(event `self.Box.OnComponentBeginOverlap`
  (params (OverlappedComponent :type "PrimitiveComponent Object Reference") (OtherActor :type "Actor Object Reference") (OtherComp :type "PrimitiveComponent Object Reference") (OtherBodyIndex :type Integer) (bFromSweep :type Boolean) (SweepResult :type "HitResult Structure (by ref)"))
  ;[1 1 1] Rotate Lilylaunchpads
  (`/Engine/EditorBlueprintResources/StandardMacros.DoOnce` false :!label _label
    (:`Completed`
      (`/Engine/EditorBlueprintResources/StandardMacros.FlipFlop`
        (:`A`
          (`self.Rotate`))
        (:`B`
          (`self.Rotate 2`))))))

(fn `UserConstructionScript`)