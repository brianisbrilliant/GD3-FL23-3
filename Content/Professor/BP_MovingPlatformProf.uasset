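; Moving platform actor that travels between Start and End component positions, starting automatically at BeginPlay.
; A Timeline, its play rate set by AnimationSpeed, drives a lerp of the Platform's relative location without sweeping.
; A FlipFlop alternates forward and reverse playback, re-triggered after WaitDelay when Looping is set, giving a back-and-forth motion with pauses.
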(event `self.ReceiveBeginPlay`
  (`TimelineComponent.SetPlayRate` (`self.Timeline`) (`self.AnimationSpeed`)) ; Wanna play
  (`/Engine/EditorBlueprintResources/StandardMacros.FlipFlop` :!label _label ; move to end, \nmove to start
    (:`A`
      (bind (_direction _newtrack_0) (`Timeline|Timeline` :!via `PlayFromStart` :!label _label_2)
        (:`Update`
          (`SceneComponent.K2_SetRelativeLocation` (`self.Platform`) (`KismetMathLibrary.VLerp` (`SceneComponent.RelativeLocation` (`self.Start`)) (`SceneComponent.RelativeLocation` (`self.End`)) _newtrack_0) false false))
        (:`Finished`
          (`KismetSystemLibrary.Delay` (`self.WaitDelay`))
          (if (`self.Looping`)
            (goto _label)))))
    (:`B`
      (goto _label_2 :!via `ReverseFromEnd`))))

(fn `UserConstructionScript`)