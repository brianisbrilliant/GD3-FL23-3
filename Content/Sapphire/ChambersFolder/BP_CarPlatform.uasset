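; BP_CarPlatform is a moving car hazard that restarts the current level when it hits the player.
; From BeginPlay it repeatedly shoves the van mesh along an Arrow component's forward vector with random-strength velocity impulses, re-triggering itself after a short delay.
; When its Box overlaps BP_Devvy, it plays a crash sound at the player and, after a brief pause, reopens the current level by name.
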(event `self.ReceiveBeginPlay`
  (`self.Push_Car`))

(event `self.Box.OnComponentBeginOverlap`
  (params (OverlappedComponent :type "PrimitiveComponent Object Reference") (OtherActor :type "Actor Object Reference") (OtherComp :type "PrimitiveComponent Object Reference") (OtherBodyIndex :type Integer) (bFromSweep :type Boolean) (SweepResult :type "HitResult Structure (by ref)"))
  (bind _asbp_devvy (cast `/Game/Blueprints/BP_Devvy` OtherActor)) ; Was it the player?
  (`GameplayStatics.PlaySoundAtLocation` "/Game/Sapphire/ChambersFolder/crash-7075.crash-7075" (`self.K2_GetActorLocation` _asbp_devvy) (struct) 1.0 1.0 0.0 null null null null)
  (`KismetSystemLibrary.Delay` 0.15)
  (bind _returnvalue (`GameplayStatics.GetCurrentLevelName` true))
  (`GameplayStatics.OpenLevel` (`KismetStringLibrary.Conv_StringToName` _returnvalue)))

(event `Push_Car`
  (bind _arrow (`self.Arrow`))
  (`PrimitiveComponent.AddVelocityChangeImpulseAtLocation` (`self.SK_Veh_Car_Van_01`) (* (`SceneComponent.GetForwardVector` _arrow) (`KismetMathLibrary.RandomFloatInRange` 200.0 350.0)) (`SceneComponent.K2_GetComponentLocation` _arrow) "None")
  (`KismetSystemLibrary.Delay` 0.5)
  (`self.Push_Car`))

(fn `UserConstructionScript`)