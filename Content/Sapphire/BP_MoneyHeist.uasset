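; BP_MoneyHeist is a pickup that adds 10 to the HUD score and destroys itself when collected.
; On BeginPlay, the Bounce timeline moves the Cylinder vertically by adding its track value to the current height each update.
; The Sphere overlap accepts BP_Devvy directly, or any actor tagged Drone, in which case it credits the player pawn's BP_Devvy HUD.
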(event `self.ReceiveBeginPlay`
  (bind _cylinder (`self.Cylinder`))
  (bind (_returnvalue_x _returnvalue_y _returnvalue_z) (`KismetMathLibrary.BreakVector` (`SceneComponent.K2_GetComponentLocation` _cylinder)))
  (bind (_direction _newtrack_0) (`Timeline|Bounce`)
    (:`Update`
      (`SceneComponent.K2_SetWorldLocation` _cylinder (`KismetMathLibrary.MakeVector` _returnvalue_x _returnvalue_y (+ _returnvalue_z (* _newtrack_0 1.0))) false false))))

(event `self.Sphere.OnComponentBeginOverlap`
  (params (OverlappedComponent :type "PrimitiveComponent Object Reference") (OtherActor :type "Actor Object Reference") (OtherComp :type "PrimitiveComponent Object Reference") (OtherBodyIndex :type Integer) (bFromSweep :type Boolean) (SweepResult :type "HitResult Structure (by ref)"))
  (if (`self.ActorHasTag` OtherActor "Drone")
    (bind _asbp_devvy (cast `/Game/Blueprints/BP_Devvy` (`GameplayStatics.GetPlayerPawn` 0)))
    (bind _hud (`/Game/Blueprints/BP_Devvy.HUD` _asbp_devvy))
    (set `/Game/Professor/W_PlayerHUD.Score` (+ (`/Game/Professor/W_PlayerHUD.Score` _hud) 10) _hud) ; Add 10 to the score
    (`self.K2_DestroyActor`)
    (else
      (bind _asbp_devvy_2 (cast `/Game/Blueprints/BP_Devvy` OtherActor))
      (bind _hud_2 (`/Game/Blueprints/BP_Devvy.HUD` _asbp_devvy_2))
      (set `/Game/Professor/W_PlayerHUD.Score` (+ (`/Game/Professor/W_PlayerHUD.Score` _hud_2) 10) _hud_2) ; Add 10 to the score
      (`self.K2_DestroyActor`))))

(fn `UserConstructionScript`)