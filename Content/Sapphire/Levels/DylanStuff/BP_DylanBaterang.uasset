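; BP_DylanBaterang is a player-steered flying projectile that takes over the camera and input on spawn, with a looping or attached sound.
; Each tick it drives the Drone's physics velocity along its aim arrow, while look axes rotate it and Sprint boosts speed.
; A forward line trace destroys it near blocking surfaces.
; Overlapping a tagged BP_Button switches that button off, returns the view to the player character and destroys the projectile.
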(event `self.ReceiveBeginPlay`
  (bind _returnvalue (`GameplayStatics.GetPlayerController` 0))
  (bind _returnvalue_2 (`GameplayStatics.SpawnSoundAttached` (`self.Sound`) (`self.Hitbox`) "None" (0.0 0.0 0.0) (struct) "KeepRelativeOffset" false 1.0 1.0 0.0 null null))
  (set `self.SpawnedSound` _returnvalue_2)
  (`self.EnableInput` _returnvalue)
  (`PlayerController.SetViewTargetWithBlend` _returnvalue self 0.0 "VTBlend_Linear" 0.0 false))

(event `InputAxis|LookUp`
  (params (AxisValue :type "Float (single-precision)"))
  (`SceneComponent.K2_AddLocalRotation` (`self.Drone`) (`KismetMathLibrary.MakeRotator` (* AxisValue 1.0)) false false))

(event `self.ReceiveTick`
  (params (DeltaSeconds :type "Float (single-precision)"))
  (bind _aimarrow (`self.aimarrow`))
  (bind _returnvalue (`SceneComponent.K2_GetComponentLocation` _aimarrow))
  (`PrimitiveComponent.SetPhysicsLinearVelocity` (`self.Drone`) (* (`SceneComponent.GetForwardVector` (`self.aimarrow`)) (`self.Speed`)) false "None")
  (bind _outhit (`KismetSystemLibrary.LineTraceSingle` _returnvalue (+ _returnvalue (* (`self.Speed`) (`SceneComponent.GetForwardVector` _aimarrow))) "TraceTypeQuery1"))
  (if (`GameplayStatics.BreakHitResult` _outhit)
    (if (< (`.Distance` (`GameplayStatics.BreakHitResult` _outhit)) 50.0)
      (`AudioComponent.Stop` (`self.SpawnedSound`))
      (`self.K2_DestroyActor`))))

(event `InputAxis|Turn`
  (params (AxisValue :type "Float (single-precision)"))
  (`SceneComponent.K2_AddLocalRotation` (`self.Drone`) (`KismetMathLibrary.MakeRotator` 0.0 0.0 AxisValue) false false))

(event `InputAction|Sprint`
  (params (Key :type "Key Structure"))
  (:`Pressed`
    (set `self.Speed` 1000.0))
  (:`Released`
    (set `self.Speed` 500.0)))

(event `self.Hitbox.OnComponentBeginOverlap`
  (params (OverlappedComponent :type "PrimitiveComponent Object Reference") (OtherActor :type "Actor Object Reference") (OtherComp :type "PrimitiveComponent Object Reference") (OtherBodyIndex :type Integer) (bFromSweep :type Boolean) (SweepResult :type "HitResult Structure (by ref)"))
  (bind _playerstate (`Controller.PlayerState` (`GameplayStatics.GetPlayerController` 0)))
  (if (`self.ActorHasTag` OtherActor "Button")
    (bind _asbp_button (cast `/Game/Sapphire/Levels/DylanStuff/BP_Button` OtherActor))
    (`/Game/Sapphire/Levels/DylanStuff/BP_Button.TurnOff` _asbp_button)
    (`self.DisableInput` (`GameplayStatics.GetPlayerController` 0))
    (`AudioComponent.Stop` (`self.SpawnedSound`))
    (`PlayerController.SetViewTargetWithBlend` (`PlayerState.GetPlayerController` _playerstate) (`GameplayStatics.GetPlayerCharacter` (`GameplayStatics.GetPlayerControllerID` (`PlayerState.GetPlayerController` _playerstate))) 0.0 "VTBlend_Linear" 0.0 false)
    (`self.K2_DestroyActor`)
    (elif (== OtherActor "/Game/Professor/BP_TestLava.BP_TestLava")
      _)))

(fn `UserConstructionScript`)