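; BP_BaterangSpawner is an actor that spawns a BP_DylanBaterang at its Arrow component's transform through an overlap trigger.
; Begin overlap on component W enters a DoOnce fed by a comparison of the other actor to the player controller, then spawns and prints a debug message.
; End overlap resets the DoOnce only if the overlapped component equals the player controller.
; A "Player" tag check is left unconnected.
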(event `self.w.OnComponentBeginOverlap`
  (params (OverlappedComponent :type "PrimitiveComponent Object Reference") (OtherActor :type "Actor Object Reference") (OtherComp :type "PrimitiveComponent Object Reference") (OtherBodyIndex :type Integer) (bFromSweep :type Boolean) (SweepResult :type "HitResult Structure (by ref)"))
  (`/Engine/EditorBlueprintResources/StandardMacros.DoOnce` (== OtherActor (`GameplayStatics.GetPlayerController` 0)) :!label _label
    (:`Completed`
      (`|SpawnActorFromClass` "/Game/Sapphire/BP_DylanBaterang.BP_DylanBaterang_C" (`SceneComponent.K2_GetComponentToWorld` (`self.Arrow`)) "Undefined" "MultiplyWithRoot" null null)
      (`KismetSystemLibrary.PrintString` "spawned"))))

(event `self.w.OnComponentEndOverlap`
  (params (OverlappedComponent :type "PrimitiveComponent Object Reference") (OtherActor :type "Actor Object Reference") (OtherComp :type "PrimitiveComponent Object Reference") (OtherBodyIndex :type Integer))
  (if (== OverlappedComponent (`GameplayStatics.GetPlayerController` 0))
    (goto _label :!via `Reset`)))

(fn `UserConstructionScript`)